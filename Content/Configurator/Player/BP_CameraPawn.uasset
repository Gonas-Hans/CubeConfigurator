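; Orbit camera pawn for the configurator, with the mouse cursor shown from BeginPlay.
; While the right mouse button is held, Turn yaws the actor and LookUp pitches the SpringArm, with no pitch clamp in the graph.
; ZoomIn and ZoomOut call a helper that respectively lengthens and shortens the arm in fixed steps within a clamped range.
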(event EventBeginPlay
  (Variables|/Script/Engine.PlayerController|SetbShowMouseCursor (Game|GetPlayerController 0) true))

(event Input|ActionEvents|InputActionZoomOut
  (params (Key :type Key%20Structure :default "None"))
  (:Pressed
    (CallFunction|ZoomArmSpring (Variables|Default|GetSpringArm) -1e+02 2e+02 2e+03)))

(event Input|ActionEvents|InputActionZoomIn
  (params (Key :type Key%20Structure :default "None"))
  (:Pressed
    (CallFunction|ZoomArmSpring (Variables|Default|GetSpringArm) 1e+02 2e+02 2e+03)))

(event Input|AxisEvents|InputAxisTurn
  (params (AxisValue :type Float%20%28single-precision%29))
  (if (Variables|Default|GetRMC)
    (Class|Actor|AddActorWorldRotation (Math|Rotator|MakeRotator 0.0 0.0 AxisValue))))

(event Input|AxisEvents|InputAxisLookUp
  (params (AxisValue :type Float%20%28single-precision%29))
  (if (Variables|Default|GetRMC)
    (Transformation|AddRelativeRotation (Variables|Default|GetSpringArm) (Math|Rotator|MakeRotator 0.0 AxisValue 0.0) false false)))

(event Input|MouseEvents|RightMouseButton
  (params (Key :type Key%20Structure :default "None"))
  (:Pressed
    (Variables|Default|SetRMC true))
  (:Released
    (Variables|Default|SetRMC false)))

(fn ConstructionScript)

(fn ZoomArmSpring
  (params (SpringComponent :type Spring%20Arm%20Component%20Object%20Reference) (ZoomValue :type Float%20%28single-precision%29) (Min :type Float%20%28single-precision%29) (Max :type Float%20%28single-precision%29))
  (Variables|/Script/Engine.SpringArmComponent|SetTargetArmLength SpringComponent (Math|Float|Clamp(Float) (+ ZoomValue (Variables|/Script/Engine.SpringArmComponent|GetTargetArmLength SpringComponent)) Min Max)))